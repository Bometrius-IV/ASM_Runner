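; BP_Drunkbot is an obstacle for the endless runner, a robot that walks along a spline.
; Each tick it advances a distance by Speed and sets the DrunkRobot component's relative transform from the spline's local transform, with fixed height and yaw offsets.
; The distance resets to zero past the spline's end, so the walk always loops; the Loop variable is unused.
; BeginPlay and construction only call the parent class.
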(event EventBeginPlay
  (|CallParentFunction))

(event Collision|EventActorBeginOverlap
  (params (OtherActor :type Actor%20Object%20Reference)))

(event EventTick
  (params (DeltaSeconds :type Float%20%28single-precision%29))
  ;[1 1 1] Walk Animation on Spline
  (Variables|Default|SetDistance%20along%20spline (+ (* DeltaSeconds (Variables|Default|GetSpeed)) (Variables|Default|GetDistance%20along%20spline)))
  (Transformation|SetRelativeTransform (Variables|Default|GetDrunk_Robot) (Math|Transform|MakeTransform (Math|Vector|MakeVector (.x (.location (Spline|GetTransformatDistanceAlongSpline (Variables|Default|GetSpline) (Variables|Default|GetDistance%20along%20spline) "Local" false))) (.y (.location (Spline|GetTransformatDistanceAlongSpline (Variables|Default|GetSpline) (Variables|Default|GetDistance%20along%20spline) "Local" false))) (+ (.z (.location (Spline|GetTransformatDistanceAlongSpline (Variables|Default|GetSpline) (Variables|Default|GetDistance%20along%20spline) "Local" false))) -2e+02)) (Math|Rotator|MakeRotator (.roll (.rotation (Spline|GetTransformatDistanceAlongSpline (Variables|Default|GetSpline) (Variables|Default|GetDistance%20along%20spline) "Local" false))) (.pitch (.rotation (Spline|GetTransformatDistanceAlongSpline (Variables|Default|GetSpline) (Variables|Default|GetDistance%20along%20spline) "Local" false))) (+ (.yaw (.rotation (Spline|GetTransformatDistanceAlongSpline (Variables|Default|GetSpline) (Variables|Default|GetDistance%20along%20spline) "Local" false))) -4e+01)) (Variables|/Script/Engine.SceneComponent|GetRelativeScale3D (Variables|Default|GetDrunk_Robot))) false false)
  (if true
    (if (> (Variables|Default|GetDistance%20along%20spline) (Spline|GetSplineLength (Variables|Default|GetSpline)))
      (Variables|Default|SetDistance%20along%20spline 0.0))))

(fn ConstructionScript
  (|CallParentFunction))