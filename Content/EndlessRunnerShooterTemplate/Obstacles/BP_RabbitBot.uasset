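; BP_RabbitBot is an endless runner obstacle actor: a rabbit robot that travels along a spline path.
; Each Tick advances the distance along the spline by Speed and sets the bot's relative transform from the local spline transform at that point.
; Fixed height and yaw offsets adjust the bot to the path while its own scale is kept.
; When Loop is enabled, the distance resets to zero past the spline's end.
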(event EventBeginPlay
  (|CallParentFunction) ; This node is disabled and will not be called.\nDrag off pins to build functionality.
)

(event Collision|EventActorBeginOverlap
  (params (OtherActor :type Actor%20Object%20Reference)))

(event EventTick
  (params (DeltaSeconds :type Float%20%28single-precision%29))
  ;[1 1 1] Walk Animation on Spline
  (Variables|Default|SetDistance%20along%20spline (+ (* DeltaSeconds (Variables|Default|GetSpeed)) (Variables|Default|GetDistance%20along%20spline)))
  (Transformation|SetRelativeTransform (Variables|Default|GetRabbit_Bot) (Math|Transform|MakeTransform (Math|Vector|MakeVector (.x (.location (Spline|GetTransformatDistanceAlongSpline (Variables|Default|GetSpline) (Variables|Default|GetDistance%20along%20spline) "Local" false))) (.y (.location (Spline|GetTransformatDistanceAlongSpline (Variables|Default|GetSpline) (Variables|Default|GetDistance%20along%20spline) "Local" false))) (+ (.z (.location (Spline|GetTransformatDistanceAlongSpline (Variables|Default|GetSpline) (Variables|Default|GetDistance%20along%20spline) "Local" false))) -3e+02)) (Math|Rotator|MakeRotator (.roll (.rotation (Spline|GetTransformatDistanceAlongSpline (Variables|Default|GetSpline) (Variables|Default|GetDistance%20along%20spline) "Local" false))) (.pitch (.rotation (Spline|GetTransformatDistanceAlongSpline (Variables|Default|GetSpline) (Variables|Default|GetDistance%20along%20spline) "Local" false))) (+ (.yaw (.rotation (Spline|GetTransformatDistanceAlongSpline (Variables|Default|GetSpline) (Variables|Default|GetDistance%20along%20spline) "Local" false))) -9e+01)) (Variables|/Script/Engine.SceneComponent|GetRelativeScale3D (Variables|Default|GetRabbit_Bot))) false false)
  (if (Variables|Default|GetLoop?)
    (if (> (Variables|Default|GetDistance%20along%20spline) (Spline|GetSplineLength (Variables|Default|GetSpline)))
      (Variables|Default|SetDistance%20along%20spline 0.0))))

(fn ConstructionScript
  (|CallParentFunction))