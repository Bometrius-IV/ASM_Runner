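; BP_Void is an endless runner obstacle that kills the player pawn on contact.
; Overlap begin and end events on its Dead component cast the other actor to BP_EndlessRunnerShooterPawnBase, set IsDead and call OnPlayerDied, so both entering and leaving trigger death.
; The construction script calls its parent and sizes the Box component from the BoxExtend variable.
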(event OnComponentBeginOverlap(Dead)
  (params (OverlappedComponent :type Primitive%20Component%20Object%20Reference) (OtherActor :type Actor%20Object%20Reference) (OtherComp :type Primitive%20Component%20Object%20Reference) (OtherBodyIndex :type Integer) (bFromSweep :type Boolean) (SweepResult :type Hit%20Result%20Structure%20%28by%20ref%29))
  (bind _asbp_endless_runner_shooter_pawn_base (Utilities|Casting|CastToBP_EndlessRunnerShooterPawnBase OtherActor))
  (Variables|/Game/EndlessRunnerShooterTemplate/Player/BP_EndlessRunnerShooterPawnBase.BP_EndlessRunnerShooterPawnBase_C|SetisDead _asbp_endless_runner_shooter_pawn_base true)
  (Default|OnPlayerDied _asbp_endless_runner_shooter_pawn_base))

(event OnComponentEndOverlap(Dead)
  (params (OverlappedComponent :type Primitive%20Component%20Object%20Reference) (OtherActor :type Actor%20Object%20Reference) (OtherComp :type Primitive%20Component%20Object%20Reference) (OtherBodyIndex :type Integer))
  (bind _asbp_endless_runner_shooter_pawn_base (Utilities|Casting|CastToBP_EndlessRunnerShooterPawnBase OtherActor))
  (Variables|/Game/EndlessRunnerShooterTemplate/Player/BP_EndlessRunnerShooterPawnBase.BP_EndlessRunnerShooterPawnBase_C|SetisDead _asbp_endless_runner_shooter_pawn_base true)
  (Default|OnPlayerDied _asbp_endless_runner_shooter_pawn_base))

(event EventBeginPlay)

(event Collision|EventActorBeginOverlap
  (params (OtherActor :type Actor%20Object%20Reference)))

(event EventTick
  (params (DeltaSeconds :type Float%20%28single-precision%29)))

(fn ConstructionScript
  (|CallParentFunction)
  (Components|Box|SetBoxExtent (Variables|Default|GetBox) (Variables|Default|GetboxExtend) true))