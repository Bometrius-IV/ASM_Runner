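; Player pawn Blueprint for an endless runner shooter, layering effects and death handling over its parent class.
; Fire plays a muzzle flash at the Gun's Muzzle socket and a gunshot sound, then calls the parent's fire logic.
; On death, it ragdolls the mesh and plays a death sound, then after a short delay shows the lose widget with UI-only input and pauses the game.
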(event Custom|PlayMuzzleFlashAndSound
  (bind _projectilespawnlocation (CallFunction|GetProjectileSpawnLocation))
  (Effects|SpawnEmitteratLocation "/Game/EndlessRunnerShooterTemplate/ParticleEffects/P_MuzzleFlash.P_MuzzleFlash" _projectilespawnlocation)
  (Audio|PlaySoundatLocation "/Game/EndlessRunnerShooterTemplate/Sounds/CUE_Gunshot.CUE_Gunshot" (Transformation|GetWorldLocation (Variables|Character|GetMesh)) "0, 0, 0" 1.0 1.0 0.0 0 0 0 0))

(event EventFire
  (CallFunction|PlayMuzzleFlashandSound)
  (|CallParentFunction))

(event EventOnPlayerDied
  (bind _returnvalue (Game|GetPlayerController 0))
  (bind _losereference (Variables|Default|GetLoseReference))
  (if (Variables|Default|GetisDead)
    (Physics|SetSimulatePhysics (Variables|Character|GetMesh) true)
    (Audio|PlaySound2D "/Game/EndlessRunnerShooterTemplate/Sounds/RowanAudio/8Bit_Death_SFX.8Bit_Death_SFX" 1.0 1.0 0.0 0 0)
    (Utilities|FlowControl|Delay 2.5)
    (Variables|/Script/Engine.PlayerController|SetbShowMouseCursor _returnvalue true)
    (Input|SetInputModeUIOnly _returnvalue _losereference "DoNotLock" false)
    (UserInterface|Viewport|AddtoViewport _losereference 0)
    (Game|SetGamePaused true)))

(fn ConstructionScript
  (|CallParentFunction))

(fn GetProjectileSpawnLocation
  (return (Transformation|GetSocketLocation (Variables|Default|GetGun) "Muzzle")))