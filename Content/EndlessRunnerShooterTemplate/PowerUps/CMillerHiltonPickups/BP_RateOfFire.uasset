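; Rate-of-fire power-up for the endless runner shooter that temporarily shortens the collecting pawn's fire cooldown.
; On collection it lowers FireCooldown, hides the pickup mesh and waits for LuckyTimer.
; It then sets the cooldown to a hardcoded value rather than the saved original, and only afterwards calls the parent OnCollected.
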(event EventBeginPlay
  (|CallParentFunction) ; This node is disabled and will not be called.\nDrag off pins to build functionality.
)

(event Collision|EventActorBeginOverlap
  (params (OtherActor :type Actor%20Object%20Reference)))

(event EventTick
  (params (DeltaSeconds :type Float%20%28single-precision%29)))

(event EventOnCollected
  (params (endlessRunnerShooterPawnBase :type BP%20Endless%20Runner%20Shooter%20Pawn%20Base%20Object%20Reference))
  (Variables|/Game/EndlessRunnerShooterTemplate/Player/BP_EndlessRunnerShooterPawnBase.BP_EndlessRunnerShooterPawnBase_C|SetfireCooldown endlessRunnerShooterPawnBase 0.2)
  (Rendering|SetVisibility (Variables|Default|GetPowerUpMesh) false false)
  (Utilities|FlowControl|Delay (Variables|Default|GetLuckyTimer))
  (Variables|/Game/EndlessRunnerShooterTemplate/Player/BP_EndlessRunnerShooterPawnBase.BP_EndlessRunnerShooterPawnBase_C|SetfireCooldown endlessRunnerShooterPawnBase 1.0)
  (|CallParentFunction 0))

(fn ConstructionScript
  (|CallParentFunction))