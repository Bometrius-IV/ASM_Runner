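; BP_SlowSpeed is an endless runner pickup that temporarily slows the pawn that collects it.
; Its OnCollected event sets the pawn's walking and crouched max speeds to a fixed reduced value.
; After a LuckyTimer delay, it sets both speeds to the pawn's RunSpeed rather than caching the previous values.
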(event EventBeginPlay
  (|CallParentFunction) ; This node is disabled and will not be called.\nDrag off pins to build functionality.
)

(event Collision|EventActorBeginOverlap
  (params (OtherActor :type Actor%20Object%20Reference)))

(event EventTick
  (params (DeltaSeconds :type Float%20%28single-precision%29)))

(event EventOnCollected
  (params (endlessRunnerShooterPawnBase :type BP%20Endless%20Runner%20Shooter%20Pawn%20Base%20Object%20Reference))
  (bind _charactermovement (Variables|/Script/Engine.Character|GetCharacterMovement endlessRunnerShooterPawnBase))
  (bind _runspeed (Variables|/Game/EndlessRunnerShooterTemplate/Player/BP_EndlessRunnerShooterPawnBase.BP_EndlessRunnerShooterPawnBase_C|GetrunSpeed endlessRunnerShooterPawnBase))
  (Variables|/Script/Engine.CharacterMovementComponent|SetMaxWalkSpeed _charactermovement 5e+02)
  (Variables|/Script/Engine.CharacterMovementComponent|SetMaxWalkSpeedCrouched _charactermovement 5e+02)
  (Utilities|FlowControl|Delay (Variables|Default|GetLuckyTimer))
  (Variables|/Script/Engine.CharacterMovementComponent|SetMaxWalkSpeed _charactermovement _runspeed)
  (Variables|/Script/Engine.CharacterMovementComponent|SetMaxWalkSpeedCrouched _charactermovement _runspeed))

(fn ConstructionScript
  (|CallParentFunction))